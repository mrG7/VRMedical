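; Blueprint function library of geometry helpers for planes in 3D space.
; GetPlaneByPoint and its pure twin compute the A, B, C, D plane equation coefficients from three points, using the cross product of two edge vectors as the normal.
; GetDistanceToPlaneByPlanePure returns a point's unsigned distance to such a plane, and GetDistanceToPlaneByPointPure chains both steps to measure directly from three points.
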(fn GetPlanebyPoint
  (params (p1 :type Vector) (p2 :type Vector) (p3 :type Vector))
  (bind (_x _y _z) (Math|Vector|BreakVector p1))
  (bind (_x_2 _y_2 _z_2) (Math|Vector|BreakVector p2))
  (bind (_x_3 _y_3 _z_3) (Math|Vector|BreakVector p3))
  (bind _returnvalue (- _y_2 _y))
  (bind _returnvalue_2 (- _z_3 _z))
  (bind _returnvalue_3 (- _z_2 _z))
  (bind _returnvalue_4 (- _y_3 _y))
  (bind _returnvalue_5 (- _x_3 _x))
  (bind _returnvalue_6 (- _x_2 _x))
  (bind _returnvalue_7 (* _returnvalue _returnvalue_2))
  (bind _returnvalue_8 (* _returnvalue_4 _returnvalue_3))
  (bind _returnvalue_9 (* _returnvalue_3 _returnvalue_5))
  (bind _returnvalue_10 (* _returnvalue_6 _returnvalue_2))
  (bind _returnvalue_11 (* _returnvalue_6 _returnvalue_4))
  (bind _returnvalue_12 (* _returnvalue _returnvalue_5))
  (bind _returnvalue_13 (- _returnvalue_7 _returnvalue_8))
  (bind _returnvalue_14 (- _returnvalue_9 _returnvalue_10))
  (bind _returnvalue_15 (- _returnvalue_11 _returnvalue_12))
  (return _returnvalue_13 _returnvalue_14 _returnvalue_15 (* (+ (+ (* _x _returnvalue_13) (* _y _returnvalue_14)) (* _z _returnvalue_15)) -1.0)))

(fn GetPlanebyPointPure
  (params (p1 :type Vector) (p2 :type Vector) (p3 :type Vector))
  (bind (_x _y _z) (Math|Vector|BreakVector p1))
  (bind (_x_2 _y_2 _z_2) (Math|Vector|BreakVector p2))
  (bind (_x_3 _y_3 _z_3) (Math|Vector|BreakVector p3))
  (bind _returnvalue (- _y_2 _y))
  (bind _returnvalue_2 (- _z_3 _z))
  (bind _returnvalue_3 (- _z_2 _z))
  (bind _returnvalue_4 (- _y_3 _y))
  (bind _returnvalue_5 (- _x_3 _x))
  (bind _returnvalue_6 (- _x_2 _x))
  (bind _returnvalue_7 (* _returnvalue _returnvalue_2))
  (bind _returnvalue_8 (* _returnvalue_4 _returnvalue_3))
  (bind _returnvalue_9 (* _returnvalue_3 _returnvalue_5))
  (bind _returnvalue_10 (* _returnvalue_6 _returnvalue_2))
  (bind _returnvalue_11 (* _returnvalue_6 _returnvalue_4))
  (bind _returnvalue_12 (* _returnvalue _returnvalue_5))
  (bind _returnvalue_13 (- _returnvalue_7 _returnvalue_8))
  (bind _returnvalue_14 (- _returnvalue_9 _returnvalue_10))
  (bind _returnvalue_15 (- _returnvalue_11 _returnvalue_12))
  (return _returnvalue_13 _returnvalue_14 _returnvalue_15 (* (+ (+ (* _x _returnvalue_13) (* _y _returnvalue_14)) (* _z _returnvalue_15)) -1.0)))

(fn GetDistancetoPlanebyPlanePure
  (params (p :type Vector) (a :type Float%20%28single-precision%29) (b :type Float%20%28single-precision%29) (c :type Float%20%28single-precision%29) (d :type Float%20%28single-precision%29))
  (bind (_x _y _z) (Math|Vector|BreakVector p))
  (return (/ (Math|Float|Absolute(Float) (+ (+ (+ (* _x a) (* _y b)) (* _z c)) d)) (Math|Float|Sqrt (+ (+ (* a a) (* b b)) (* c c))))))

(fn GetDistancetoPlanebyPointPure
  (params (p :type Vector) (p1 :type Vector) (p2 :type Vector) (p3 :type Vector))
  (bind (_a _b _c _d) (CallFunction|GetPlanebyPointPure p1 p2 p3))
  (return (CallFunction|GetDistancetoPlanebyPlanePure p _a _b _c _d)))