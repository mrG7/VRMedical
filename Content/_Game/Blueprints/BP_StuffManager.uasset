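; Manages eight anatomical system models (body, skeleton, muscle and others), moving them between combined and separated layouts.
; Tweens snap each child actor's transform to its own billboard or the shared combine billboard, including when dismissed from the platform.
; For attached models, it isolates a named sub-mesh at a platform point, shrinking the rest and setting the player's scale speed.
; Tag widget visibility follows attached and combined state.
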(event Custom|Combine
  (|CombineAllParts)
  (Utilities|UpdateAllTagVisibility))

(event Custom|FirstShow
  (|ShowHideAllParts false
    (:Completed
      (Rendering|SetVisibility (Variables|Default|Getbody) true true)
      (Utilities|FlowControl|Delay 3.0)
      (|ShowHideAllParts_2 true))))

(event Custom|Separate
  (|SeparateAllParts)
  (Utilities|UpdateAllTagVisibility
    (:Completed
      (bind _asbp_player (Utilities|Casting|CastToBP_Player (Game|Player|GetPlayerPawn 0)))
      (bind _aswbp_hand_menu_ui (Utilities|Casting|CastToWBP_HandMenuUI (UserInterface|GetUserWidgetObject (Variables|/Game/_Game/Blueprints/BP_Player.BP_Player_C|GetWidgetLeft _asbp_player))))
      (Default|OnSeperateSystem _aswbp_hand_menu_ui))))

(event EventBeginPlay
  (|InitialAllParts)
  (Utilities|UpdateAllTagVisibility))

(fn ConstructionScript)

(fn DismissfromPlatform
  (params (Type :type BPE_System%20Enum))
  (switch Utilities|FlowControl|Switch|SwitchonBPE_System Type
    (:NewEnumerator0
      (CallFunction|SetSnapTarget (Variables|Default|Getbody)))
    (:NewEnumerator1
      (CallFunction|SetSnapTarget (Variables|Default|Getcirculatory)))
    (:NewEnumerator2
      (CallFunction|SetSnapTarget (Variables|Default|Getlymph)))
    (:NewEnumerator3
      (CallFunction|SetSnapTarget (Variables|Default|Getmuscle)))
    (:NewEnumerator4
      (CallFunction|SetSnapTarget (Variables|Default|Getnerve)))
    (:NewEnumerator5
      (CallFunction|SetSnapTarget (Variables|Default|Getskeleton)))
    (:NewEnumerator6
      (CallFunction|SetSnapTarget (Variables|Default|Geturinary)))
    (:NewEnumerator7
      (CallFunction|SetSnapTarget (Variables|Default|Getviscera)))))

(fn SetSnapTarget
  (params (SystemRef :type Child%20Actor%20Component%20Object%20Reference))
  (bind _childactor (Variables|/Script/Engine.ChildActorComponent|GetChildActor SystemRef))
  (bind _asbp_man_base (Utilities|Casting|CastToBP_ManBase _childactor))
  (if (Variables|Params|GetIsCombined)
    (LocalVariables|SetBilliboardRef (Variables|/Game/_Game/Blueprints/BP_ManBase.BP_ManBase_C|GetCombineBilliboard _asbp_man_base))
    (else
      (LocalVariables|SetBilliboardRef (Variables|/Game/_Game/Blueprints/BP_ManBase.BP_ManBase_C|GetSeperateBilliboard _asbp_man_base))))
  (Default|ShowTagWidget _asbp_man_base)
  (Transformation|DetachFromActor _childactor "KeepWorld" "KeepWorld" "KeepWorld")
  (Variables|/Game/_Game/Blueprints/BP_ManBase.BP_ManBase_C|SetIsAttached _asbp_man_base false)
  (Utilities|Snapfromto _childactor (LocalVariables|GetBilliboardRef) "None" 1.0)
  (return))

(fn ShowOneSubSystem
  (params (Name :type String))
  (bind (_lefts _rights) (Utilities|String|Split Name "#"))
  (bind _returnvalue (Game|Player|GetPlayerPawn 0))
  (bind _platformref (Variables|Setup|GetPlatformRef))
  (bind (_asbp_player _bsuccess) (Utilities|Casting|CastToBP_Player _returnvalue))
  (LocalVariables|SetPartName _lefts)
  (LocalVariables|SetSubName _rights)
  (Transformation|SetRelativeScale3D (Variables|/Game/_Game/Blueprints/BP_RotatePlatform.BP_RotatePlatform_C|GetPlatformScale _platformref) "1.000000,1.000000,1.000000")
  (Transformation|SetRelativeScale3D (Variables|/Game/_Game/Blueprints/BP_RotatePlatform.BP_RotatePlatform_C|GetStuff _platformref) "1.000000,1.000000,1.000000")
  (for _array_element (Variables|Params|GetAllParts)
    ;[1 1 1] 遍历所有Actor
    (LocalVariables|SetCurrentActor (Variables|/Script/Engine.ChildActorComponent|GetChildActor _array_element))
    (if (Variables|/Game/_Game/Blueprints/BP_ManBase.BP_ManBase_C|GetIsAttached (.AsBP%20Man%20Base (Utilities|Casting|CastToBP_ManBase (Variables|/Script/Engine.ChildActorComponent|GetChildActor _array_element))))
      (if (Utilities|Enum|Equal(Enum) (Utilities|GetObjectName _array_element) (LocalVariables|GetPartName))
        (Transformation|SetActorRelativeScale3D (LocalVariables|GetCurrentActor) "1.000000,1.000000,1.000000")
        (for _array_element_2 (Components|GetChildrenComponents (VehicleSound|GetRootComponent (LocalVariables|GetCurrentActor)) false)
          ;[1 1 1] 遍历所有Component
          (bind _asstatic_mesh_component (Utilities|Casting|CastToStaticMeshComponent _array_element_2))
          (if (Utilities|String|Contains (Utilities|GetObjectName _asstatic_mesh_component) (LocalVariables|GetSubName))
            (if (!= (Variables|Params|GetCurrentSubMeshComp) 0)
              (Transformation|SetRelativeLocation (Variables|Params|GetCurrentSubMeshComp) (Variables|Params|GetCurSubCompOriginLoc) false false))
            (Variables|Params|SetCurrentSubMeshComp _asstatic_mesh_component)
            (Variables|Params|SetCurSubCompOriginLoc (Variables|/Script/Engine.SceneComponent|GetRelativeLocation (Variables|Params|GetCurrentSubMeshComp)))
            (Class|ITween|ComponentMovefromtoSimple "No Name" (Variables|Params|GetCurrentSubMeshComp) (Transformation|GetWorldLocation (Variables|Params|GetCurrentSubMeshComp)) (CallFunction|GetSubSystemAssignLoc) "world" false 0.3 "linear")
            (Class|ITween|ComponentScalefromtoSimple "No Name" (Variables|Params|GetCurrentSubMeshComp) (Variables|/Script/Engine.SceneComponent|GetRelativeScale3D (Variables|Params|GetCurrentSubMeshComp)) "1.000000,1.000000,1.000000" false 0.3 "linear")
            (Variables|/Game/_Game/Blueprints/BP_Player.BP_Player_C|SetIsScaleSubSystem _asbp_player _bsuccess)
            (if (Components|ComponentHasTag (Variables|Params|GetCurrentSubMeshComp) "SubSystemAssignButtom")
              (Variables|/Game/_Game/Blueprints/BP_Player.BP_Player_C|SetScaleSpeed _asbp_player (Variables|Setup|GetScaleSpeedSlow))
              (else
                (Variables|/Game/_Game/Blueprints/BP_Player.BP_Player_C|SetScaleSpeed _asbp_player (Variables|Setup|GetScaleSpeedFast))))
            (else
              (Class|ITween|ComponentScalefromtoSimple "No Name" _asstatic_mesh_component (Variables|/Script/Engine.SceneComponent|GetRelativeScale3D _asstatic_mesh_component) "0.000000,0.000000,0.000000" false 0.3 "linear"))))
        (else
          (Class|ITween|ActorScalefromtoSimple "No Name" (LocalVariables|GetCurrentActor) (Class|Actor|GetActorRelativeScale3D (LocalVariables|GetCurrentActor)) "0.000000,0.000000,0.000000" false 0.3 "linear")))))
  (Utilities|UpdateAllTagVisibility))

(fn GetSubSystemAssignLoc
  (if (Components|ComponentHasTag (Variables|Params|GetCurrentSubMeshComp) "SubSystemAssignButtom")
    (LocalVariables|SetReLoc (Transformation|GetWorldLocation (Variables|/Game/_Game/Blueprints/BP_RotatePlatform.BP_RotatePlatform_C|GetSubSystemPointDown (Variables|Setup|GetPlatformRef))))
    (else
      (LocalVariables|SetReLoc (Transformation|GetWorldLocation (Variables|/Game/_Game/Blueprints/BP_RotatePlatform.BP_RotatePlatform_C|GetSubSystemPointUp (Variables|Setup|GetPlatformRef))))))
  (return (LocalVariables|GetReLoc)))

(fn ShowPartSystem
  (bind _returnvalue (Game|Player|GetPlayerPawn 0))
  (bind _platformref (Variables|Setup|GetPlatformRef))
  (bind _asbp_player (Utilities|Casting|CastToBP_Player _returnvalue))
  (Variables|/Game/_Game/Blueprints/BP_Player.BP_Player_C|SetIsScaleSubSystem _asbp_player false)
  (Variables|/Game/_Game/Blueprints/BP_Player.BP_Player_C|SetScaleSpeed _asbp_player (Variables|Setup|GetScaleSpeedSlow))
  (Transformation|SetRelativeScale3D (Variables|/Game/_Game/Blueprints/BP_RotatePlatform.BP_RotatePlatform_C|GetPlatformScale _platformref) "1.000000,1.000000,1.000000")
  (Transformation|SetRelativeScale3D (Variables|/Game/_Game/Blueprints/BP_RotatePlatform.BP_RotatePlatform_C|GetStuff _platformref) "1.000000,1.000000,1.000000")
  (for _array_element (Variables|Params|GetAllParts)
    ;[1 1 1] 遍历所有Actor
    (LocalVariables|SetCurrentActor (Variables|/Script/Engine.ChildActorComponent|GetChildActor _array_element))
    (if (Variables|/Game/_Game/Blueprints/BP_ManBase.BP_ManBase_C|GetIsAttached (.AsBP%20Man%20Base (Utilities|Casting|CastToBP_ManBase (Variables|/Script/Engine.ChildActorComponent|GetChildActor _array_element))))
      (Transformation|SetActorRelativeScale3D (LocalVariables|GetCurrentActor) "1.000000,1.000000,1.000000")))
  (if (!= (Variables|Params|GetCurrentSubMeshComp) 0)
    (Transformation|SetRelativeLocation (Variables|Params|GetCurrentSubMeshComp) (Variables|Params|GetCurSubCompOriginLoc) false false)
    (for _array_element_2 (Components|GetChildrenComponents (VehicleSound|GetRootComponent (Components|GetOwner (Variables|Params|GetCurrentSubMeshComp))) false)
      ;[1 1 1] 遍历所有Component
      (bind _asstatic_mesh_component (Utilities|Casting|CastToStaticMeshComponent _array_element_2))
      (Transformation|SetRelativeScale3D _asstatic_mesh_component "1.000000,1.000000,1.000000"))
    (Variables|Params|SetCurrentSubMeshComp 0)
    (Utilities|UpdateAllTagVisibility)))