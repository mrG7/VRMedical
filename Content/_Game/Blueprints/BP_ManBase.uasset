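; Base actor for an exhibit that flies onto the rotating observation platform and registers its system type in the player's hand menu.
; On BeginPlay it caches the first BP_RotatePlatform in the level.
; AttachToPlatform tweens location, rotation and scale to the platform's Stuff component, then, after a matching delay, snap-attaches to it.
; It then hides the tag widget, flags itself attached and updates the left-hand menu.
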(event Custom|ShowTagWidget
  (bind _widget (Variables|Default|GetWidget))
  (Collision|SetCollisionEnabled _widget "QueryAndPhysics")
  (Rendering|SetVisibility _widget true true))

(event Custom|HideTagWidget
  (bind _widget (Variables|Default|GetWidget))
  (Collision|SetCollisionEnabled _widget "NoCollision")
  (Rendering|SetVisibility _widget false true))

(event Custom|AttachToPlatform
  (bind _self self)
  ;[1 1 1] 附着到观察平台
  (Class|ITween|ActorMovefromtoSimple "No Name" _self (.Loaction (|From-Transform)) (.Location (Math|Conversions|ToTransform(Vector))) "world" false 1.0 "linear")
  (Class|ITween|ActorRotatefromtoSimple "No Name" _self (.Rotation (|From-Transform_2)) (.Rotation (|To-Transform_2)) "world" false 1.0 "linear")
  (Class|ITween|ActorScalefromtoSimple "No Name" _self (.Scale (|From-Transform_3)) (.Scale (|To-Transform_3)) false 1.0 "linear")
  (Utilities|FlowControl|Delay 1.0)
  (Transformation|AttachComponentToComponent (Variables|/Game/_Game/Blueprints/BP_RotatePlatform.BP_RotatePlatform_C|GetStuff (Variables|Default|GetPlatform)) "None" "SnapToTarget" "SnapToTarget" "SnapToTarget" false)
  (CallFunction|HideTagWidget)
  (Variables|Setup|SetIsAttached true)
  (CallFunction|AddtoHandMenu))

(event EventBeginPlay
  (bind _outactors (Actor|GetAllActorsOfClass "/Game/_Game/Blueprints/BP_RotatePlatform.BP_RotatePlatform_C"))
  (Variables|Default|SetPlatform (Utilities|Array|Get(acopy) _outactors)))

(fn ConstructionScript)

(fn AddtoHandMenu
  (bind _aswbp_hand_menu_ui (Utilities|Casting|CastToWBP_HandMenuUI (UserInterface|GetUserWidgetObject (Variables|/Game/_Game/Blueprints/BP_Player.BP_Player_C|GetWidgetLeft (.AsBP%20Player (Utilities|Casting|CastToBP_Player (Game|Player|GetPlayerPawn 0)))))))
  (Default|AddOnetoMenu _aswbp_hand_menu_ui (Variables|Setup|GetSystemType)))